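; BP_IceSpwan is a spawner that keeps creating BP_Ice actors at random points inside its Box component.
; From BeginPlay, it runs an endless cycle that alternates two short For loops with Delay nodes, the last Delay wiring back to the first loop.
; Since loops do not wait on Delays, each cycle spawns one ice, pauses, spawns two together, then pauses again.
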(event `self.ReceiveBeginPlay`
  (bind _box (`self.Box`))
  (bind _box_2 (`self.Box`))
  (for _ (range 1) :!label _label
    (`|SpawnActorFromClass` "/Game/IceCatch/BP_Ice.BP_Ice_C" (`KismetMathLibrary.MakeTransform` (`KismetMathLibrary.RandomPointInBoundingBox` (`SceneComponent.K2_GetComponentLocation` _box_2) (`BoxComponent.BoxExtent` _box_2))) "Undefined" "OverrideRootScale" null null)
    (`KismetSystemLibrary.Delay` 7.0)
    (for _ (range 2)
      (`|SpawnActorFromClass` "/Game/IceCatch/BP_Ice.BP_Ice_C" (`KismetMathLibrary.MakeTransform` (`KismetMathLibrary.RandomPointInBoundingBox` (`SceneComponent.K2_GetComponentLocation` _box) (`BoxComponent.BoxExtent` _box))) "Undefined" "OverrideRootScale" null null)
      (`KismetSystemLibrary.Delay` 3.0)
      (goto _label))))

(fn `UserConstructionScript`)